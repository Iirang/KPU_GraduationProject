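; BP_Minimap is a minimap actor that puts a Wdg_Minimap widget on screen at BeginPlay and carries a SceneCaptureComponent2D.
; Every Tick it sets its location to player character 0's position multiplied by (0, 0, 2), zeroing X and Y and doubling Z.
; An unconnected chain that would attach the capture component above the player with world rotation kept never runs.
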(event `self.ReceiveBeginPlay`
  (bind _returnvalue (`|CreateWidget` "/Game/Minimap/Wdg_Minimap.Wdg_Minimap_C"))
  (`UserWidget.AddToViewport` _returnvalue 0))

(event `self.ReceiveTick`
  (params (DeltaSeconds :type "Float (single-precision)"))
  ;[1 1 1] 미니맵 회전 값을 고정시켜 놓는 것
  ; AttachToComponent 값이 BeginPlay와 연결이 되어있으면 안된다.
  (`self.K2_SetActorLocation` (* (`self.K2_GetActorLocation` (`GameplayStatics.GetPlayerCharacter` 0)) (0.0 0.0 2.0))))

(fn `UserConstructionScript`)