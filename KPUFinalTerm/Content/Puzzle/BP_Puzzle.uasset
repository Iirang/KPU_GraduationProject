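; Nine-plate stepping puzzle in the style of Lights Out, where the ThirdPersonCharacter sinks plates by walking onto them.
; BeginPlay caches each cube's raised and lowered locations.
; Overlapping a raised plate lowers it and toggles hard-wired linked plates via MoveComponentTo, updating per-plate Overlap and Success flags; Success is never read here.
; A reset trigger raises all cubes but leaves those flags unchanged.
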(event `self.ReceiveBeginPlay`
  (`self.PuzzleLocation`))

(event `self.Cube_Collision_1.OnComponentBeginOverlap`
  (params (OverlappedComponent :type "PrimitiveComponent Object Reference") (OtherActor :type "Actor Object Reference") (OtherComp :type "PrimitiveComponent Object Reference") (OtherBodyIndex :type Integer) (bFromSweep :type Boolean) (SweepResult :type "HitResult Structure (by ref)"))
  ;[1 1 1] 첫번째 발판 / 1>4
  (if (== (`GameplayStatics.GetObjectClass` OtherActor) "/Game/Character/Blueprints/ThirdPersonCharacter.ThirdPersonCharacter_C")
    (if (not (`self.b1PuzzleOverlap`))
      (`|ExecutionSequence`
        (:`then_0`
          (set `self.b1PuzzleOverlap` true)
          (`KismetSystemLibrary.MoveComponentTo` (`self.Cube_Puzzle_1`) (`self.1PuzzleDownLocation`) (struct) false false 1.0)
          (set `self.b1PuzzleSuccess` true))
        (:`then_1`
          (if (`self.b4PuzzleOverlap`)
            (`KismetSystemLibrary.MoveComponentTo` (`self.Cube_Puzzle_4`) (`self.4PuzzleUpLocation`) (struct) false false 1.0)
            (set `self.b4PuzzleOverlap` false)
            (set `self.b4PuzzleSuccess` false)
            (else
              (`KismetSystemLibrary.MoveComponentTo` (`self.Cube_Puzzle_4`) (`self.4PuzzleDownLocation`) (struct) false false 1.0)
              (set `self.b4PuzzleSuccess` true)
              (set `self.b4PuzzleSuccess` true))))))))

(event `self.Cube_Collision_6.OnComponentBeginOverlap`
  (params (OverlappedComponent :type "PrimitiveComponent Object Reference") (OtherActor :type "Actor Object Reference") (OtherComp :type "PrimitiveComponent Object Reference") (OtherBodyIndex :type Integer) (bFromSweep :type Boolean) (SweepResult :type "HitResult Structure (by ref)"))
  ;[1 1 1] 여섯번째 발판 / 6>5
  (if (== (`GameplayStatics.GetObjectClass` OtherActor) "/Game/Character/Blueprints/ThirdPersonCharacter.ThirdPersonCharacter_C")
    (if (not (`self.b6PuzzleOverlap`))
      (`|ExecutionSequence`
        (:`then_0`
          (set `self.b6PuzzleOverlap` true)
          (`KismetSystemLibrary.MoveComponentTo` (`self.Cube_Puzzle_6`) (`self.6PuzzleDownLocation`) (struct) false false 1.0)
          (set `self.b6PuzzleSuccess` true))
        (:`then_1`
          (if (`self.b5PuzzleOverlap`)
            (`KismetSystemLibrary.MoveComponentTo` (`self.Cube_Puzzle_5`) (`self.5PuzzleUpLocation`) (struct) false false 1.0)
            (set `self.b5PuzzleOverlap` false)
            (set `self.b5PuzzleSuccess` false)
            (else
              (`KismetSystemLibrary.MoveComponentTo` (`self.Cube_Puzzle_5`) (`self.5PuzzleDownLocation`) (struct) false false 1.0)
              (set `self.b5PuzzleOverlap` true)
              (set `self.b5PuzzleSuccess` true))))))))

(event `self.ResetCubeCollison.OnComponentBeginOverlap`
  (params (OverlappedComponent :type "PrimitiveComponent Object Reference") (OtherActor :type "Actor Object Reference") (OtherComp :type "PrimitiveComponent Object Reference") (OtherBodyIndex :type Integer) (bFromSweep :type Boolean) (SweepResult :type "HitResult Structure (by ref)"))
  (if (== (`GameplayStatics.GetObjectClass` OtherActor) "/Game/Character/Blueprints/ThirdPersonCharacter.ThirdPersonCharacter_C")
    (`|ExecutionSequence`
      (:`then_0`
        (`KismetSystemLibrary.MoveComponentTo` (`self.Cube_Puzzle_1`) (`self.1PuzzleUpLocation`) (struct) false false 1.0))
      (:`then_1`
        (`KismetSystemLibrary.MoveComponentTo` (`self.Cube_Puzzle_2`) (`self.2PuzzleUpLocation`) (struct) false false 1.0))
      (:`then_2`
        (`KismetSystemLibrary.MoveComponentTo` (`self.Cube_Puzzle_3`) (`self.3PuzzleUpLocation`) (struct) false false 1.0))
      (:`then_3`
        (`KismetSystemLibrary.MoveComponentTo` (`self.Cube_Puzzle_4`) (`self.4PuzzleUpLocation`) (struct) false false 1.0))
      (:`then_4`
        (`KismetSystemLibrary.MoveComponentTo` (`self.Cube_Puzzle_5`) (`self.5PuzzleUpLocation`) (struct) false false 1.0))
      (:`then_5`
        (`KismetSystemLibrary.MoveComponentTo` (`self.Cube_Puzzle_6`) (`self.6PuzzleUpLocation`) (struct) false false 1.0))
      (:`then_6`
        (`KismetSystemLibrary.MoveComponentTo` (`self.Cube_Puzzle_7`) (`self.7PuzzleUpLocation`) (struct) false false 1.0))
      (:`then_7`
        (`KismetSystemLibrary.MoveComponentTo` (`self.Cube_Puzzle_8`) (`self.8PuzzleUpLocation`) (struct) false false 1.0))
      (:`then_8`
        (`KismetSystemLibrary.MoveComponentTo` (`self.Cube_Puzzle_9`) (`self.9PuzzleUpLocation`) (struct) false false 1.0)))))

(event `self.Cube_Collision_2.OnComponentBeginOverlap`
  (params (OverlappedComponent :type "PrimitiveComponent Object Reference") (OtherActor :type "Actor Object Reference") (OtherComp :type "PrimitiveComponent Object Reference") (OtherBodyIndex :type Integer) (bFromSweep :type Boolean) (SweepResult :type "HitResult Structure (by ref)"))
  ;[1 1 1] 두번째 발판 / 2>4
  (if (== (`GameplayStatics.GetObjectClass` OtherActor) "/Game/Character/Blueprints/ThirdPersonCharacter.ThirdPersonCharacter_C")
    (if (not (`self.b2PuzzleOverlap`))
      (`|ExecutionSequence`
        (:`then_0`
          (set `self.b2PuzzleOverlap` true)
          (`KismetSystemLibrary.MoveComponentTo` (`self.Cube_Puzzle_2`) (`self.2PuzzleDownLocation`) (struct) false false 1.0)
          (set `self.b2PuzzleSuccess` true))
        (:`then_1`
          (if (`self.b4PuzzleOverlap`)
            (`KismetSystemLibrary.MoveComponentTo` (`self.Cube_Puzzle_4`) (`self.4PuzzleUpLocation`) (struct) false false 1.0)
            (set `self.b4PuzzleOverlap` false)
            (set `self.b4PuzzleSuccess` false)
            (else
              (`KismetSystemLibrary.MoveComponentTo` (`self.Cube_Puzzle_4`) (`self.4PuzzleDownLocation`) (struct) false false 1.0)
              (set `self.b4PuzzleOverlap` true)
              (set `self.b4PuzzleSuccess` true))))))))

(event `self.Cube_Collision_7.OnComponentBeginOverlap`
  (params (OverlappedComponent :type "PrimitiveComponent Object Reference") (OtherActor :type "Actor Object Reference") (OtherComp :type "PrimitiveComponent Object Reference") (OtherBodyIndex :type Integer) (bFromSweep :type Boolean) (SweepResult :type "HitResult Structure (by ref)"))
  ;[1 1 1] 일곱번째 발판 / 7>8
  (if (== (`GameplayStatics.GetObjectClass` OtherActor) "/Game/Character/Blueprints/ThirdPersonCharacter.ThirdPersonCharacter_C")
    (if (not (`self.b7PuzzleOverlap`))
      (`|ExecutionSequence`
        (:`then_0`
          (set `self.b7PuzzleOverlap` true)
          (`KismetSystemLibrary.MoveComponentTo` (`self.Cube_Puzzle_7`) (`self.7PuzzleDownLocation`) (struct) false false 1.0)
          (set `self.b7PuzzleSuccess` true))
        (:`then_1`
          (if (`self.b8PuzzleOverlap`)
            (`KismetSystemLibrary.MoveComponentTo` (`self.Cube_Puzzle_8`) (`self.8PuzzleUpLocation`) (struct) false false 1.0)
            (set `self.b8PuzzleOverlap` false)
            (set `self.b8PuzzleSuccess` false)
            (else
              (`KismetSystemLibrary.MoveComponentTo` (`self.Cube_Puzzle_8`) (`self.8PuzzleDownLocation`) (struct) false false 1.0)
              (set `self.b8PuzzleOverlap` true)
              (set `self.b8PuzzleSuccess` true))))))))

(event `self.Cube_Collision_3.OnComponentBeginOverlap`
  (params (OverlappedComponent :type "PrimitiveComponent Object Reference") (OtherActor :type "Actor Object Reference") (OtherComp :type "PrimitiveComponent Object Reference") (OtherBodyIndex :type Integer) (bFromSweep :type Boolean) (SweepResult :type "HitResult Structure (by ref)"))
  ;[1 1 1] 세번째 발판 / 3>2
  (if (== (`GameplayStatics.GetObjectClass` OtherActor) "/Game/Character/Blueprints/ThirdPersonCharacter.ThirdPersonCharacter_C")
    (if (not (`self.b3PuzzleOverlap`))
      (`|ExecutionSequence`
        (:`then_0`
          (set `self.b3PuzzleOverlap` true)
          (`KismetSystemLibrary.MoveComponentTo` (`self.Cube_Puzzle_3`) (`self.3PuzzleDownLocation`) (struct) false false 1.0)
          (set `self.b3PuzzleSuccess` true))
        (:`then_1`
          (if (`self.b2PuzzleOverlap`)
            (`KismetSystemLibrary.MoveComponentTo` (`self.Cube_Puzzle_2`) (`self.2PuzzleUpLocation`) (struct) false false 1.0)
            (set `self.b2PuzzleOverlap` false)
            (set `self.b2PuzzleSuccess` false)
            (else
              (`KismetSystemLibrary.MoveComponentTo` (`self.Cube_Puzzle_2`) (`self.2PuzzleDownLocation`) (struct) false false 1.0)
              (set `self.b2PuzzleOverlap` true)
              (set `self.b2PuzzleSuccess` true))))))))

(event `self.Cube_Collision_8.OnComponentBeginOverlap`
  (params (OverlappedComponent :type "PrimitiveComponent Object Reference") (OtherActor :type "Actor Object Reference") (OtherComp :type "PrimitiveComponent Object Reference") (OtherBodyIndex :type Integer) (bFromSweep :type Boolean) (SweepResult :type "HitResult Structure (by ref)"))
  ;[1 1 1] 여덟번째 발판 / 8>6
  (if (== (`GameplayStatics.GetObjectClass` OtherActor) "/Game/Character/Blueprints/ThirdPersonCharacter.ThirdPersonCharacter_C")
    (if (not (`self.b8PuzzleOverlap`))
      (`|ExecutionSequence`
        (:`then_0`
          (set `self.b8PuzzleOverlap` true)
          (`KismetSystemLibrary.MoveComponentTo` (`self.Cube_Puzzle_8`) (`self.8PuzzleDownLocation`) (struct) false false 1.0)
          (set `self.b8PuzzleSuccess` true))
        (:`then_1`
          (if (`self.b6PuzzleOverlap`)
            (`KismetSystemLibrary.MoveComponentTo` (`self.Cube_Puzzle_6`) (`self.6PuzzleUpLocation`) (struct) false false 1.0)
            (set `self.b6PuzzleOverlap` false)
            (set `self.b6PuzzleSuccess` false)
            (else
              (`KismetSystemLibrary.MoveComponentTo` (`self.Cube_Puzzle_6`) (`self.6PuzzleDownLocation`) (struct) false false 1.0)
              (set `self.b6PuzzleOverlap` true)
              (set `self.b6PuzzleSuccess` true))))))))

(event `self.Cube_Collision_4.OnComponentBeginOverlap`
  (params (OverlappedComponent :type "PrimitiveComponent Object Reference") (OtherActor :type "Actor Object Reference") (OtherComp :type "PrimitiveComponent Object Reference") (OtherBodyIndex :type Integer) (bFromSweep :type Boolean) (SweepResult :type "HitResult Structure (by ref)"))
  ;[1 1 1] 네번째 발판 / 4>2 / 4>8
  (if (== (`GameplayStatics.GetObjectClass` OtherActor) "/Game/Character/Blueprints/ThirdPersonCharacter.ThirdPersonCharacter_C")
    (if (not (`self.b4PuzzleOverlap`))
      (`|ExecutionSequence`
        (:`then_0`
          (set `self.b4PuzzleOverlap` true)
          (`KismetSystemLibrary.MoveComponentTo` (`self.Cube_Puzzle_4`) (`self.4PuzzleDownLocation`) (struct) false false 1.0)
          (set `self.b4PuzzleSuccess` true))
        (:`then_1`
          (if (`self.b2PuzzleOverlap`)
            (`KismetSystemLibrary.MoveComponentTo` (`self.Cube_Puzzle_2`) (`self.2PuzzleUpLocation`) (struct) false false 1.0)
            (set `self.b2PuzzleOverlap` false)
            (set `self.b2PuzzleSuccess` false)
            (else
              (`KismetSystemLibrary.MoveComponentTo` (`self.Cube_Puzzle_2`) (`self.2PuzzleDownLocation`) (struct) false false 1.0)
              (set `self.b2PuzzleOverlap` true)
              (set `self.b2PuzzleSuccess` true))))
        (:`then_2`
          (if (`self.b8PuzzleOverlap`)
            (`KismetSystemLibrary.MoveComponentTo` (`self.Cube_Puzzle_8`) (`self.8PuzzleUpLocation`) (struct) false false 1.0)
            (set `self.b8PuzzleOverlap` false)
            (set `self.b8PuzzleSuccess` false)
            (else
              (`KismetSystemLibrary.MoveComponentTo` (`self.Cube_Puzzle_8`) (`self.8PuzzleDownLocation`) (struct) false false 1.0)
              (set `self.b8PuzzleOverlap` true)
              (set `self.b8PuzzleSuccess` true))))))))

(event `self.Cube_Collision_9.OnComponentBeginOverlap`
  (params (OverlappedComponent :type "PrimitiveComponent Object Reference") (OtherActor :type "Actor Object Reference") (OtherComp :type "PrimitiveComponent Object Reference") (OtherBodyIndex :type Integer) (bFromSweep :type Boolean) (SweepResult :type "HitResult Structure (by ref)"))
  ;[1 1 1] 아홉번째 발판 / 9>6
  (if (== (`GameplayStatics.GetObjectClass` OtherActor) "/Game/Character/Blueprints/ThirdPersonCharacter.ThirdPersonCharacter_C")
    (if (not (`self.b9PuzzleOverlap`))
      (`|ExecutionSequence`
        (:`then_0`
          (set `self.b9PuzzleOverlap` true)
          (`KismetSystemLibrary.MoveComponentTo` (`self.Cube_Puzzle_9`) (`self.9PuzzleDownLocation`) (struct) false false 1.0)
          (set `self.b9PuzzleSuccess` true))
        (:`then_1`
          (if (`self.b6PuzzleOverlap`)
            (`KismetSystemLibrary.MoveComponentTo` (`self.Cube_Puzzle_6`) (`self.6PuzzleUpLocation`) (struct) false false 1.0)
            (set `self.b6PuzzleOverlap` false)
            (set `self.b6PuzzleSuccess` false)
            (else
              (`KismetSystemLibrary.MoveComponentTo` (`self.Cube_Puzzle_6`) (`self.6PuzzleDownLocation`) (struct) false false 1.0)
              (set `self.b6PuzzleOverlap` true)
              (set `self.b6PuzzleSuccess` true))))))))

(event `self.Cube_Collision_5.OnComponentBeginOverlap`
  (params (OverlappedComponent :type "PrimitiveComponent Object Reference") (OtherActor :type "Actor Object Reference") (OtherComp :type "PrimitiveComponent Object Reference") (OtherBodyIndex :type Integer) (bFromSweep :type Boolean) (SweepResult :type "HitResult Structure (by ref)"))
  ;[1 1 1] 5번째 발판 / 5>2/5>4/5>6/5>8
  (if (== (`GameplayStatics.GetObjectClass` OtherActor) "/Game/Character/Blueprints/ThirdPersonCharacter.ThirdPersonCharacter_C")
    (if (not (`self.b5PuzzleOverlap`))
      (`|ExecutionSequence`
        (:`then_0`
          (set `self.b5PuzzleOverlap` true)
          (`KismetSystemLibrary.MoveComponentTo` (`self.Cube_Puzzle_5`) (`self.5PuzzleDownLocation`) (struct) false false 1.0)
          (set `self.b5PuzzleSuccess` true))
        (:`then_1`
          (if (`self.b2PuzzleOverlap`)
            (`KismetSystemLibrary.MoveComponentTo` (`self.Cube_Puzzle_2`) (`self.2PuzzleUpLocation`) (struct) false false 1.0)
            (set `self.b2PuzzleOverlap` false)
            (set `self.b2PuzzleSuccess` false)
            (else
              (`KismetSystemLibrary.MoveComponentTo` (`self.Cube_Puzzle_2`) (`self.2PuzzleDownLocation`) (struct) false false 1.0)
              (set `self.b2PuzzleOverlap` true)
              (set `self.b2PuzzleSuccess` true))))
        (:`then_2`
          (if (`self.b4PuzzleOverlap`)
            (`KismetSystemLibrary.MoveComponentTo` (`self.Cube_Puzzle_4`) (`self.4PuzzleUpLocation`) (struct) false false 1.0)
            (set `self.b4PuzzleOverlap` false)
            (set `self.b4PuzzleSuccess` false)
            (else
              (`KismetSystemLibrary.MoveComponentTo` (`self.Cube_Puzzle_4`) (`self.4PuzzleDownLocation`) (struct) false false 1.0)
              (set `self.b4PuzzleOverlap` true)
              (set `self.b4PuzzleSuccess` true))))
        (:`then_3`
          (if (`self.b6PuzzleOverlap`)
            (`KismetSystemLibrary.MoveComponentTo` (`self.Cube_Puzzle_6`) (`self.6PuzzleUpLocation`) (struct) false false 1.0)
            (set `self.b6PuzzleOverlap` false)
            (set `self.b6PuzzleSuccess` false)
            (else
              (`KismetSystemLibrary.MoveComponentTo` (`self.Cube_Puzzle_6`) (`self.6PuzzleDownLocation`) (struct) false false 1.0)
              (set `self.b6PuzzleOverlap` true)
              (set `self.b6PuzzleSuccess` true))))
        (:`then_4`
          (if (`self.b8PuzzleOverlap`)
            (`KismetSystemLibrary.MoveComponentTo` (`self.Cube_Puzzle_8`) (`self.8PuzzleUpLocation`) (struct) false false 1.0)
            (set `self.b8PuzzleOverlap` false)
            (set `self.b8PuzzleSuccess` false)
            (else
              (`KismetSystemLibrary.MoveComponentTo` (`self.Cube_Puzzle_8`) (`self.8PuzzleDownLocation`) (struct) false false 1.0)
              (set `self.b8PuzzleOverlap` true)
              (set `self.b8PuzzleSuccess` true))))))))

(fn `1PuzzleLocation`
  (bind _relativelocation (`SceneComponent.RelativeLocation` (`self.Cube_Puzzle_1`)))
  (set `self.1PuzzleUpLocation` _relativelocation)
  (set `self.1PuzzleDownLocation` (- _relativelocation (0.0 0.0 35.0))))

(fn `2PuzzleLocation`
  (bind _relativelocation (`SceneComponent.RelativeLocation` (`self.Cube_Puzzle_2`)))
  (set `self.2PuzzleUpLocation` _relativelocation)
  (set `self.2PuzzleDownLocation` (- _relativelocation (0.0 0.0 35.0))))

(fn `3PuzzleLocation`
  (bind _relativelocation (`SceneComponent.RelativeLocation` (`self.Cube_Puzzle_3`)))
  (set `self.3PuzzleUpLocation` _relativelocation)
  (set `self.3PuzzleDownLocation` (- _relativelocation (0.0 0.0 35.0))))

(fn `4PuzzleLocation`
  (bind _relativelocation (`SceneComponent.RelativeLocation` (`self.Cube_Puzzle_4`)))
  (set `self.4PuzzleUpLocation` _relativelocation)
  (set `self.4PuzzleDownLocation` (- _relativelocation (0.0 0.0 35.0))))

(fn `5PuzzleLocation`
  (bind _relativelocation (`SceneComponent.RelativeLocation` (`self.Cube_Puzzle_5`)))
  (set `self.5PuzzleUpLocation` _relativelocation)
  (set `self.5PuzzleDownLocation` (- _relativelocation (0.0 0.0 35.0))))

(fn `6PuzzleLocation`
  (bind _relativelocation (`SceneComponent.RelativeLocation` (`self.Cube_Puzzle_6`)))
  (set `self.6PuzzleUpLocation` _relativelocation)
  (set `self.6PuzzleDownLocation` (- _relativelocation (0.0 0.0 35.0))))

(fn `7PuzzleLocation`
  (bind _relativelocation (`SceneComponent.RelativeLocation` (`self.Cube_Puzzle_7`)))
  (set `self.7PuzzleUpLocation` _relativelocation)
  (set `self.7PuzzleDownLocation` (- _relativelocation (0.0 0.0 35.0))))

(fn `8PuzzleLocation`
  (bind _relativelocation (`SceneComponent.RelativeLocation` (`self.Cube_Puzzle_8`)))
  (set `self.8PuzzleUpLocation` _relativelocation)
  (set `self.8PuzzleDownLocation` (- _relativelocation (0.0 0.0 35.0))))

(fn `9PuzzleLocation`
  (bind _relativelocation (`SceneComponent.RelativeLocation` (`self.Cube_Puzzle_9`)))
  (set `self.9PuzzleUpLocation` _relativelocation)
  (set `self.9PuzzleDownLocation` (- _relativelocation (0.0 0.0 35.0))))

(fn `PuzzleLocation`
  (`self.1PuzzleLocation`)
  (`self.2PuzzleLocation`)
  (`self.3PuzzleLocation`)
  (`self.4PuzzleLocation`)
  (`self.5PuzzleLocation`)
  (`self.6PuzzleLocation`)
  (`self.7PuzzleLocation`)
  (`self.8PuzzleLocation`)
  (`self.9PuzzleLocation`))

(fn `UserConstructionScript`)