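; BP_RedPuzzle_Cube is a puzzle cube that reacts to ThirdPersonCharacter overlapping its OverlapCollision.
; After a short delay, it moves Cube below the actor's location on begin overlap and above on end, gated by RedPuzzleCubeOverlap.
; Relative move targets are computed from world actor location.
; It then tries setting RedUp on BP_BluePuzzle_Cube by casting the overlapping actor, already checked as the character class, so that cast cannot succeed.
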(event `self.OverlapCollision.OnComponentBeginOverlap`
  (params (OverlappedComponent :type "PrimitiveComponent Object Reference") (OtherActor :type "Actor Object Reference") (OtherComp :type "PrimitiveComponent Object Reference") (OtherBodyIndex :type Integer) (bFromSweep :type Boolean) (SweepResult :type "HitResult Structure (by ref)"))
  (if (== (`GameplayStatics.GetObjectClass` OtherActor) "/Game/Character/Blueprints/ThirdPersonCharacter.ThirdPersonCharacter_C")
    (if (== (`self.bRedPuzzleCubeOverlap`) false)
      (`KismetSystemLibrary.Delay` 0.2)
      (`KismetSystemLibrary.MoveComponentTo` (`self.Cube`) (- (`self.K2_GetActorLocation`) (0.0 0.0 35.0)) (struct) false false 1.0)
      (set `self.bRedPuzzleCubeOverlap` true)
      (bind _asbp_blue_puzzle_cube (cast `/Game/Puzzle/BP_BluePuzzle_Cube` OtherActor))
      (set `/Game/Puzzle/BP_BluePuzzle_Cube.bRedUp` true _asbp_blue_puzzle_cube))))

(event `self.OverlapCollision.OnComponentEndOverlap`
  (params (OverlappedComponent :type "PrimitiveComponent Object Reference") (OtherActor :type "Actor Object Reference") (OtherComp :type "PrimitiveComponent Object Reference") (OtherBodyIndex :type Integer))
  (if (== (`GameplayStatics.GetObjectClass` OtherActor) "/Game/Character/Blueprints/ThirdPersonCharacter.ThirdPersonCharacter_C")
    (if (== (`self.bRedPuzzleCubeOverlap`) true)
      (`KismetSystemLibrary.Delay` 0.2)
      (`KismetSystemLibrary.MoveComponentTo` (`self.Cube`) (+ (`self.K2_GetActorLocation`) (0.0 0.0 35.0)) (struct) false false 1.0)
      (set `self.bRedPuzzleCubeOverlap` false)
      (bind _asbp_blue_puzzle_cube (cast `/Game/Puzzle/BP_BluePuzzle_Cube` OtherActor))
      (set `/Game/Puzzle/BP_BluePuzzle_Cube.bRedUp` false _asbp_blue_puzzle_cube))))

(fn `UserConstructionScript`)