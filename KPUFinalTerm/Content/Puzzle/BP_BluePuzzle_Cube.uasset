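; Blue puzzle cube actor that slides down when the third-person character enters its overlap collision and back up when they leave.
; Lowering on overlap requires RedUp to be false; this file only reads that flag.
; Tick also polls RedUp against BluePuzzleCubeOverlap, firing each move once through DoOnce gates that are never reset.
; Moves use delayed MoveComponentTo, passing actor location plus or minus a Z offset as relative location.
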(event `self.ReceiveTick`
  (params (DeltaSeconds :type "Float (single-precision)"))
  (`|ExecutionSequence`
    (:`then_0`
      (if (not (`self.bBluePuzzleCubeOverlap`))
        (if (`self.bRedUp`)
          (`KismetSystemLibrary.Delay` 0.2)
          (`/Engine/EditorBlueprintResources/StandardMacros.DoOnce` false
            (:`Completed`
              (`KismetSystemLibrary.MoveComponentTo` (`self.Cube`) (+ (`self.K2_GetActorLocation`) (0.0 0.0 35.0)) (struct) false false 1.0)
              (set `self.bBluePuzzleCubeOverlap` false))))))
    (:`then_1`
      (if (`self.bBluePuzzleCubeOverlap`)
        (if (not (`self.bRedUp`))
          (`KismetSystemLibrary.Delay` 0.2)
          (`/Engine/EditorBlueprintResources/StandardMacros.DoOnce` false
            (:`Completed`
              (`KismetSystemLibrary.MoveComponentTo` (`self.Cube`) (- (`self.K2_GetActorLocation`) (0.0 0.0 35.0)) (struct) false false 1.0)
              (set `self.bBluePuzzleCubeOverlap` true))))))))

(event `self.OverlapCollision.OnComponentBeginOverlap`
  (params (OverlappedComponent :type "PrimitiveComponent Object Reference") (OtherActor :type "Actor Object Reference") (OtherComp :type "PrimitiveComponent Object Reference") (OtherBodyIndex :type Integer) (bFromSweep :type Boolean) (SweepResult :type "HitResult Structure (by ref)"))
  (if (== (`GameplayStatics.GetObjectClass` OtherActor) "/Game/Character/Blueprints/ThirdPersonCharacter.ThirdPersonCharacter_C")
    (if (not (`self.bRedUp`))
      (if (== (`self.bBluePuzzleCubeOverlap`) false)
        (`KismetSystemLibrary.Delay` 0.2)
        (`KismetSystemLibrary.MoveComponentTo` (`self.Cube`) (- (`self.K2_GetActorLocation`) (0.0 0.0 35.0)) (struct) false false 1.0)
        (set `self.bBluePuzzleCubeOverlap` true)))))

(event `self.OverlapCollision.OnComponentEndOverlap`
  (params (OverlappedComponent :type "PrimitiveComponent Object Reference") (OtherActor :type "Actor Object Reference") (OtherComp :type "PrimitiveComponent Object Reference") (OtherBodyIndex :type Integer))
  (if (== (`GameplayStatics.GetObjectClass` OtherActor) "/Game/Character/Blueprints/ThirdPersonCharacter.ThirdPersonCharacter_C")
    (if (== (`self.bBluePuzzleCubeOverlap`) true)
      (`KismetSystemLibrary.Delay` 0.2)
      (`KismetSystemLibrary.MoveComponentTo` (`self.Cube`) (+ (`self.K2_GetActorLocation`) (0.0 0.0 35.0)) (struct) false false 1.0)
      (set `self.bBluePuzzleCubeOverlap` false))))

(fn `UserConstructionScript`)